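; Horror monster that always faces the player and periodically teleports to the TargetPoint whose distance from the player best matches TargetDistance.
; TargetDistance grows while the player sprints and shrinks while they stand still.
; That distance, or the real one when close, drives a material-collection "bubbliness" value that also sets white noise volume.
; A line trace plus facing dot product triggers a scare sound when the monster enters view, with a cooldown.
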(event EventBeginPlay
  (bind _returnvalue (Game|Player|GetPlayerPawn 0))
  ;[1 1 1] Startup
  ;;[1 1 1] Get References to Player
  (Variables|Default|SetPlayer _returnvalue)
  (bind _ascharacter (Utilities|Casting|CastToCharacter _returnvalue)
    (:then
      (Variables|Default|SetPlayerMovement (Pawn|GetMovementComponent _ascharacter))
      ;;[1 1 1] Get All Target Points
      (bind _outactors (Actor|GetAllActorsOfClass "/Script/Engine.TargetPoint"))
      (for (_array_element _array_index) _outactors
        (bind _astargetpoint (Utilities|Casting|CastToTargetPoint _array_element)
          (:then
            (Utilities|Array|Insert (Variables|Default|GetAllTargetPoints) _astargetpoint _array_index))
          (:CastFailed
            (Development|PrintString "ERROR: TargetPoint Actor was somehow not a TargetPoint!" true true "(R=1.000000,G=1.000000,B=1.000000,A=1.000000)"))))
      ;;[1 1 1] Start Monster Position Update Loop
      (Utilities|Time|SetTimerbyFunctionName 0 "Move Monster To Best Target Point" 4.25 true)
      ;;[1 1 1] Remember the Original Target Distance
      (Variables|Monster|SetMax%20Target%20Distance (Variables|Monster|GetTargetDistance)))
    (:CastFailed
      (Development|PrintString "ERROR: Player isn't a Pawn!" true true "(R=1.000000,G=1.000000,B=1.000000,A=1.000000)"))))

(event EventTick
  (params (DeltaSeconds :type Float%20%28single-precision%29))
  ;[1 1 1] Update Logic
  (Utilities|FlowControl|Sequence
    (:then_0
      ;;[1 1 1] Rotate to Face Player
      (Transformation|SetActorRotation (Math|Rotator|FindLookatRotation (Transformation|GetActorLocation) (Transformation|GetActorLocation (Variables|Default|GetPlayer)))))
    (:then_1
      ;;[1 1 1] Update Target Distance
      (if (> (Math|Vector|VectorLength (Variables|/Script/Engine.MovementComponent|GetVelocity (Variables|Default|GetPlayerMovement))) 1.0)
        (bind _issprinting_ (CallFunction|IsPlayerSprinting?))
        (if _issprinting_
          (Variables|Monster|SetTargetDistance (+ (Variables|Monster|GetTargetDistance) (* DeltaSeconds (Variables|Monster|GetTargetDistanceIncreaseRate)))))
        (else
          (Variables|Monster|SetTargetDistance (- (Variables|Monster|GetTargetDistance) (* DeltaSeconds (Variables|Monster|GetTargetDistanceDecreaseRate)))))))
    (:then_2
      ;;[1 1 1] Set Bubbliness of Materials
      (Rendering|Material|SetScalarParameterValue "/Game/Materials/BubblinessParams.BubblinessParams" "BubblyLerp" (- 1.0 (Math|Float|Clamp(Float) (/ (CallFunction|GetGraphicalTargetDistance) (Variables|Monster|GetMax%20Target%20Distance)))) :!class /Script/Engine.KismetMaterialLibrary))
    (:then_3
      ;;[1 1 1] If Monster Just Became Visible, Play Horror Sound
      (if (CallFunction|CanSeePlayer?)
        (if (Variables|Default|GetPlayerCanSeeMe?)
          (Variables|Default|SetMonsterNoiseCounter 1e+01)
          (else
            (Variables|Default|SetPlayerCanSeeMe? true)
            (if (<= (Variables|Default|GetMonsterNoiseCounter) 0.0)
              (Variables|Default|SetMonsterNoiseCounter 1e+01)
              (Class|GameplayStatics|PlaySoundAttached "/Game/Audio/SeeMonster_Cue.SeeMonster_Cue" (Variables|Default|GetMonster%20Mesh) "None" "0, 0, 0" "KeepWorldPosition")
              (else
                (Variables|Default|SetMonsterNoiseCounter 1e+01)))))
        (else
          (Variables|Default|SetMonsterNoiseCounter (- (Variables|Default|GetMonsterNoiseCounter) DeltaSeconds))
          (Variables|Default|SetPlayerCanSeeMe? false))))
    (:then_4
      ;;[1 1 1] Update Monster's White Noise
      (bind _returnvalue (Rendering|Material|GetScalarParameterValue "/Game/Materials/BubblinessParams.BubblinessParams" "BubblyLerp" :!class /Script/Engine.KismetMaterialLibrary))
      (Audio|Components|Audio|SetVolumeMultiplier (Variables|Default|GetWhiteNoise) (Math|Float|Power _returnvalue 1e+01) :!class /Script/Engine.AudioComponent))))

(fn ConstructionScript)

(fn FindBestTarget
  (bind _variable (|LocalVariable))
  (bind _variable_2 (|LocalVariable))
  (|Assign _variable -1)
  (|Assign _variable_2 -1.0)
  (for _index (range 0 (- (Utilities|Array|Length (Variables|Default|GetAllTargetPoints)) 1))
    (bind _returnvalue (Transformation|GetDistanceTo (Variables|Default|GetPlayer) (Utilities|Array|Get(acopy) (Variables|Default|GetAllTargetPoints) _index)))
    (bind _distance (CallFunction|PlayerDistancetoTargetDistance _returnvalue))
    (if (or (== _variable -1) (< _distance _variable_2))
      (|Assign _variable _index)
      (|Assign _variable_2 _distance)))
  (return (Utilities|Array|Get(acopy) (Variables|Default|GetAllTargetPoints) _variable)))

(fn PlayerDistancetoTargetDistance
  (params (PlayerDistance :type Float%20%28single-precision%29))
  (return (Math|Float|Absolute(Float) (- PlayerDistance (Variables|Monster|GetTargetDistance)))))

(fn MoveMonstertoBestTargetPoint
  (bind _besttarget (CallFunction|FindBestTarget))
  (Transformation|SetActorLocation (Transformation|GetActorLocation _besttarget) false))

(fn IsPlayerSprinting?
  (bind _ashorrorplayerchar_c (Utilities|Casting|CastToHorrorPlayerChar (Variables|Default|GetPlayer))
    (:then
      (return (Variables|/Game/Blueprints/HorrorPlayerChar.HorrorPlayerChar_C|GetIs%20Sprinting? _ashorrorplayerchar_c)))
    (:CastFailed
      (Development|PrintString "ERROR in \"MonsterBP::IsPlayerSprinting?\": Player isn't a HorrorPlayerChar instance!" true true "(R=0.000000,G=0.691991,B=0.825000,A=1.000000)"))))

(fn CanSeePlayer?
  (bind _variable (|LocalVariable))
  (bind _player (Variables|Default|GetPlayer))
  ;[1 1 1] Raycast from Player to Monster
  (bind (_outhit _returnvalue) (Collision|LineTraceForObjects (Transformation|GetActorLocation (Variables|Default|GetPlayer)) (Transformation|GetActorLocation) (Utilities|Array|MakeArray "ObjectTypeQuery1" "ObjectTypeQuery3" "ObjectTypeQuery4" "ObjectTypeQuery2") true (Utilities|Array|MakeArray (Variables|Default|GetPlayer)) "None" false))
  (Utilities|Casting|CastToMonsterBP (.HitActor (Collision|BreakHitResult _outhit))
    (:then
      (|Assign _variable (and (> (Math|Vector|DotProduct (Math|Vector|Normalize (- (Transformation|GetActorLocation) (Transformation|GetActorLocation _player))) (Transformation|GetActorForwardVector _player)) 0.4) _returnvalue)))
    (:CastFailed
      (|Assign _variable false)))
  (return _variable))

(fn GetGraphicalTargetDistance
  (bind _variable (|LocalVariable))
  (bind _returnvalue (Transformation|GetDistanceTo (Variables|Default|GetPlayer)))
  (if (> _returnvalue 5e+02)
    (|Assign _variable (Variables|Monster|GetTargetDistance))
    (else
      (|Assign _variable _returnvalue)))
  (return _variable))